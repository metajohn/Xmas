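; Test actor for the Interactable interface that damages whoever interacts with it and changes its cube's color.
; Each interaction increments InteractionInt, whose RepNotify cycles the cube through four materials.
; It also applies fixed damage through the interactor's HealthComponent, with debug prints of health before and after.
; Only the after-damage print is gated on authority; the damage call is not.
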(event OnInteracted(Interactable)
  (params (Interactor :type Actor%20Object%20Reference))
  (bind _returnvalue (Actor|GetComponentbyClass Interactor "/Script/Xmas.HealthComponent"))
  (bind _returnvalue_2 (Class|HealthComponent|GetCurrentHealth _returnvalue))
  (Development|PrintString "ButtonPressed")
  (bind _result (Math|Integer|IncrementInt (Variables|Default|GetInteractionInt))
    (:%20%20
      (Variables|Default|SetInteractionInt _result)
      (Utilities|IsValid _returnvalue
        (:Is%20Valid
          (Development|PrintString (Utilities|String|Append "Health Before Damage" (Utilities|String|ToString(Float) _returnvalue_2)))
          (Class|HealthComponent|ApplyDamage _returnvalue 1e+02 self)
          (Networking|SwitchHasAuthority
            (:Authority
              (Development|PrintString (Utilities|String|Append "Health After Damage" (Utilities|String|ToString(Float) _returnvalue_2))))))
        (:Is%20Not%20Valid
          (Development|PrintString "Health Component Is Invalid"))))))

(event EventBeginPlay)

(event Collision|EventActorBeginOverlap
  (params (OtherActor :type Actor%20Object%20Reference)))

(event EventTick
  (params (DeltaSeconds :type Float%20%28single-precision%29)))

(fn ConstructionScript)

(fn OnRepInteractionInt
  (bind _cube (Variables|Default|GetCube))
  (switch int (Math|Integer|%(Integer) (Variables|Default|GetInteractionInt) 4)
    (:0
      (Rendering|Material|SetMaterial _cube 0 "/InterchangeAssets/gltf/M_Default.M_Default"))
    (:1
      (Rendering|Material|SetMaterial _cube 0 "/AnimationSharing/AnimSharingBlue.AnimSharingBlue"))
    (:2
      (Rendering|Material|SetMaterial _cube 0 "/AnimationSharing/AnimSharingGreen.AnimSharingGreen"))
    (:3
      (Rendering|Material|SetMaterial _cube 0 "/DatasmithContent/Materials/AliasReference.AliasReference"))))